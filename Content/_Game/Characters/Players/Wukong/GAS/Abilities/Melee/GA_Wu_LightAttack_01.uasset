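; Wukong's first light melee attack, a Gameplay Ability that costs stamina and can only activate when the player has enough.
; On activation it commits, ending on failure, and applies the stamina drain effect through a SetByCaller magnitude because the cost is set at runtime.
; Montage tag notify begin and end events add and remove the combo tag on the owning character, marking the combo window.
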(event `self.OnAbilityActivatedBlueprint`
  (`|ExecutionSequence`
    (:`then_0`
      ;[1 1 1 0.5] Commit ability, lock in cost and effects upfront
      (bind _returnvalue (`self.K2_CommitAbility`))
      ;[1 1 1 0.5] If commit fails then we end ability
      (if (not _returnvalue)
        (`self.K2_EndAbility`)))
    (:`then_1`
      ;[1 1 1 0.5] Apply stamina reduction effect
      ; * Our effect requires us to set the magnitude at runtime, so we don't get the benefit of "Commit Ability" doing it all for us. Here we set the magnitude using the local variables, this will apply the stamina drain.
      (bind _staminareductioneffect (`self.StaminaReductionEffect`)
        (:`then`
          (bind _returnvalue_2 (`AbilitySystemBlueprintLibrary.AssignTagSetByCallerMagnitude` (`self.MakeOutgoingGameplayEffectSpec` _staminareductioneffect) (`self.StaminaReductionEffectTag`) (`self.StaminaCost`)))
          (`self.K2_ApplyGameplayEffectSpecToOwner` _returnvalue_2))
        (:`else`)))))

(event `self.OnTagNotifyBeginBlueprint`
  (params (Data :type "GameplayEventData Structure"))
  ;[1 1 1 0.5] Handle when playing montage hits one of our custom Anim Notify begin
  (`|SwitchGameplayTag` (`.EventTag` (break `GameplayEventData` Data))
    (:`Combat.Melee.Attack.Combo`
      ;;[1 1 1 0.5] If it's our combo lets add tag to our owning character
      (bind _cachedcharacter (`self.CachedCharacter`)
        (:`then`
          (`PGAS_CharacterBase.AddGameplayTag` _cachedcharacter (struct :`TagName` "Combat.Melee.Attack.Combo")))
        (:`else`)))))

(event `self.OnTagNotifyEndBlueprint`
  (params (Data :type "GameplayEventData Structure"))
  ;[1 1 1 0.5] Handle when playing montage hits one of our custom Anim Notify end
  (`|SwitchGameplayTag` (`.EventTag` (break `GameplayEventData` Data))
    (:`Combat.Melee.Attack.Combo`
      ;;[1 1 1 0.5] If it's our combo lets remove tag to our owning character
      (bind _cachedcharacter (`self.CachedCharacter`)
        (:`then`
          (`PGAS_CharacterBase.RemoveGameplayTag` _cachedcharacter (struct :`TagName` "Combat.Melee.Attack.Combo")))
        (:`else`)))))

(fn `DebugEventText`
  (params (EventName :type Text) (GameplayTag :type "GameplayTag Structure") (Hand :type "EPGAS_WeaponHand Enum" :default "Left"))
  (`KismetSystemLibrary.PrintText` (`|FormatText` "{Message}:  {Tag} | {Hand}" EventName (`BlueprintGameplayTagLibrary.GetTagName` GameplayTag) (`|GenericToText` Hand)) true true (struct :`A` 1.0) 5.0))

(fn `K2_CanActivateAbility`
  (params (ActorInfo :type "GameplayAbilityActorInfo Structure") (Handle :type "GameplayAbilitySpecHandle Structure"))
  (returns (RelevantTags :type "GameplayTagContainer Structure") (ReturnValue :type Boolean))
  ;[1 1 1 0.5] Make sure we have enough  stamina to perform this ability.
  ; * Cached Character pointer is already set by this time, so we can safely use it.
  (bind _aspgas_player_character (cast `PGAS_PlayerCharacter` (`self.CachedCharacter`)))
  (if (>= (`PGAS_PlayerCharacter.GetStamina` _aspgas_player_character) (`self.MakePositive` (`self.StaminaCost`)))
    (return (struct) true)
    (else
      (return (struct) false))))