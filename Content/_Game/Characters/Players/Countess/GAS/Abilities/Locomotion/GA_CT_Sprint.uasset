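; GA_CT_Sprint is the Countess's hold-to-sprint gameplay ability in GAS.
; On activation it commits, applies a stamina reduction effect to the owner, raises MaxWalkSpeed to sprint speed and adds the Sprinting tag.
; It ends when input is released, restoring walk speed, removing the tag and removing the stamina effect by its stored handle.
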(event `self.K2_ActivateAbility`
  (`|ExecutionSequence`
    (:`then_0`
      ;[1 1 1 0.5] Commit ability, lock in cost and effects upfront
      (bind _returnvalue (`self.K2_CommitAbility`))
      ;[1 1 1 0.5] If commit fails then we end ability
      (if (not _returnvalue)
        (`self.K2_EndAbility`)))
    (:`then_1`
      ;[1 1 1 0.5] Get and apply effect to owner of this ability.
      ; * Using the Jogging effect, duration = Infinite, so will apply to owner while ability is active.
      (bind _staminareductioneffect (`self.StaminaReductionEffect`)
        (:`then`
          (bind _returnvalue_2 (`self.BP_ApplyGameplayEffectToOwner` _staminareductioneffect))
          ;[1 1 1 0.5] Store handle
          (set `self.StaminaEffectHandle` _returnvalue_2))
        (:`else`)))
    (:`then_2`
      ;[1 1 1 0.5] Update character speed
      (`self.UpdateCharacterSpeed` (`self.CharacterSprintSpeed`))
      ;[1 1 1 0.5] Place tag on character
      (`self.AddGameplayTag` (struct :`TagName` "Character.Movement.Sprinting"))
      ;[1 1 1 0.5] Wait for player to release the key/gamepad button to end the ability
      (`AbilityTask_WaitInputRelease.WaitInputRelease` false
        (:`OnRelease`
          ;;[1 1 1 0.5] End Ability
          (`self.K2_EndAbility`))))))

(event `self.K2_OnEndAbility`
  (params (bWasCancelled :type Boolean))
  ;[1 1 1 0.5] Update character speed
  (`self.UpdateCharacterSpeed` (`self.CharacterWalkSpeed`))
  ;[1 1 1 0.5] Remove tag from character
  (`self.RemoveGameplayTag` (struct :`TagName` "Character.Movement.Sprinting"))
  ;[1 1 1 0.5] Remove the stamina effect from owner
  (`self.BP_RemoveGameplayEffectFromOwnerWithHandle` (`self.StaminaEffectHandle`)))

(fn `UpdateCharacterSpeed`
  (params (Speed :type "Float (double-precision)"))
  (bind _cachedcharactermovement (`self.CachedCharacterMovement`)
    (:`then`
      (set `CharacterMovementComponent.MaxWalkSpeed` Speed _cachedcharactermovement))
    (:`else`)))