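; Gameplay Ability that makes the Countess player character jump at a stamina cost.
; CanActivate checks that the cached character has enough stamina to cover the magnitude.
; Activation commits the ability, applies the stamina reduction effect with a runtime SetByCaller magnitude, calls Jump and plays a sound at the character.
; It ends immediately afterwards rather than waiting for landing, so it can activate again.
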(event `self.K2_ActivateAbility`
  (`|ExecutionSequence`
    (:`then_0`
      ;[1 1 1 0.5] Commit ability, lock in cost and effects upfront
      (bind _returnvalue (`self.K2_CommitAbility`))
      ;[1 1 1 0.5] If commit fails then we end ability
      (if (not _returnvalue)
        (`self.K2_EndAbility`)))
    (:`then_1`
      ;[1 1 1 0.5] Apply stamina reduction effect
      ; * Our effect requires us to set the magnitude at runtime, so we don't get the benefit of "Commit Ability" doing it all for us. Here we set the magnitude using the local variables, this will apply the stamina drain.
      (bind _staminareductioneffect (`self.StaminaReductionEffect`)
        (:`then`
          (bind _returnvalue_2 (`AbilitySystemBlueprintLibrary.AssignTagSetByCallerMagnitude` (`self.MakeOutgoingGameplayEffectSpec` _staminareductioneffect) (`self.StaminaReductionEffectTag`) (`self.StaminaMagnitude`)))
          (`self.K2_ApplyGameplayEffectSpecToOwner` _returnvalue_2))
        (:`else`)))
    (:`then_2`
      ;[1 1 1 0.5] Character Jump
      (bind _cachedcharacter (`self.CachedCharacter`)
        (:`then`
          (`Character.Jump` _cachedcharacter))
        (:`else`)))
    (:`then_3`
      ;[1 1 1 0.5] Play sound cue
      (bind _cachedcharacter_2 (`self.CachedCharacter`)
        (:`then`
          (`GameplayStatics.PlaySoundAtLocation` (`self.SoundEffect`) (`Actor.K2_GetActorLocation` _cachedcharacter_2) (struct) 1.0 1.0 0.0 null null null null))
        (:`else`)))
    (:`then_4`
      ;[1 1 1 0.5] Must end abilities or GAS thinks the ability is still going and you will not be able to jump again
      (`self.K2_EndAbility`))))

(event `self.K2_OnEndAbility`
  (params (bWasCancelled :type Boolean))
  (`parent.K2_OnEndAbility` bWasCancelled))

(fn `K2_CanActivateAbility`
  (params (ActorInfo :type "GameplayAbilityActorInfo Structure") (Handle :type "GameplayAbilitySpecHandle Structure"))
  (returns (RelevantTags :type "GameplayTagContainer Structure") (ReturnValue :type Boolean))
  ;[1 1 1 0.5] Make sure we have enough  stamina to perform this ability.
  ; * Cached Character pointer is already set by this time, so we can safely use it.
  (bind _aspgas_player_character (cast `PGAS_PlayerCharacter` (`self.CachedCharacter`)))
  (if (>= (`PGAS_PlayerCharacter.GetStamina` _aspgas_player_character) (`self.MakePositive` (`self.StaminaMagnitude`)))
    (return (struct) true)
    (else
      (return (struct) false))))