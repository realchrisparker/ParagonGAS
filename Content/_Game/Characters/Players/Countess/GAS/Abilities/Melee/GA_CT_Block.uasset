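; Countess gameplay ability for a hold-to-block that drains stamina and only activates when the character has at least the configured stamina magnitude.
; On activation it commits, applies a stamina effect with a SetByCaller magnitude set at runtime, adds the Combat.Blocking tag and calls StartBlocking for the AnimInstance.
; Input release ends the ability, which removes the tag and stamina effect and calls StopBlocking.
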(event `self.K2_ActivateAbility`
  (`|ExecutionSequence`
    (:`then_0`
      ;[1 1 1 0.5] Commit ability, lock in cost and effects upfront
      (bind _returnvalue (`self.K2_CommitAbility`))
      ;[1 1 1 0.5] If commit fails then we end ability
      (if (not _returnvalue)
        (`self.K2_EndAbility`)))
    (:`then_1`
      ;[1 1 1 0.5] Apply stamina reduction effect
      ; * Our effect requires us to set the magnitude at runtime, so we don't get the benefit of "Commit Ability" doing it all for us. Here we set the magnitude using the local variables, this will apply the stamina drain.
      (bind _staminareductioneffect (`self.StaminaReductionEffect`)
        (:`then`
          (bind _returnvalue_2 (`AbilitySystemBlueprintLibrary.AssignTagSetByCallerMagnitude` (`self.MakeOutgoingGameplayEffectSpec` _staminareductioneffect) (`self.StaminaReductionEffectTag`) (`self.StaminaMagnitude`)))
          (bind _returnvalue_3 (`self.K2_ApplyGameplayEffectSpecToOwner` _returnvalue_2))
          (set `self.StaminaEffectHandle` _returnvalue_3))
        (:`else`)))
    (:`then_2`
      ;[1 1 1 0.5] Place tag on character
      (`self.AddGameplayTag` (struct :`TagName` "Combat.Blocking"))
      ;[1 1 1 0.5] Tell listening AnimInstance to block. (Uses C++ Interface in this  helper function)
      (`PGAS_CharacterBase.StartBlocking` (`self.CachedCharacter`))
      ;[1 1 1 0.5] Wait for player to release the key/gamepad button to end the ability
      (`AbilityTask_WaitInputRelease.WaitInputRelease` false
        (:`OnRelease`
          ;;[1 1 1 0.5] End Ability
          (`self.K2_EndAbility`))))))

(event `self.K2_OnEndAbility`
  (params (bWasCancelled :type Boolean))
  ;[1 1 1 0.5] Remove tag from character
  (`self.RemoveGameplayTag` (struct :`TagName` "Combat.Blocking"))
  ;[1 1 1 0.5] Tell listening AnimInstance to block. (Uses C++ Interface in this  helper function)
  (`PGAS_CharacterBase.StopBlocking` (`self.CachedCharacter`))
  ;[1 1 1 0.5] Remove the stamina effect from owner
  (`self.BP_RemoveGameplayEffectFromOwnerWithHandle` (`self.StaminaEffectHandle`)))

(fn `K2_CanActivateAbility`
  (params (ActorInfo :type "GameplayAbilityActorInfo Structure") (Handle :type "GameplayAbilitySpecHandle Structure"))
  (returns (RelevantTags :type "GameplayTagContainer Structure") (ReturnValue :type Boolean))
  ;[1 1 1 0.5] Make sure we have enough  stamina to perform this ability.
  ; * Cached Character pointer is already set by this time, so we can safely use it.
  (bind _aspgas_player_character (cast `PGAS_PlayerCharacter` (`self.CachedCharacter`)))
  (if (>= (`PGAS_PlayerCharacter.GetStamina` _aspgas_player_character) (`self.MakePositive` (`self.StaminaMagnitude`)))
    (return (struct) true)
    (else
      (return (struct) false))))